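; BP_TestActor is a test actor for trying out click-driven RPCs and property replication.
; On BeginPlay it binds a click handler, which prints the clicked actor's name and passes it to TestRpc on the first BP_TestPlayerController.
; RepNotify functions for RepBool and RepActor print their values with debug tags.
; A TestBlueprintCallable call and a BeginPlay debug print are left unconnected.
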(event Custom|OnClicked_Event
  (params (TouchedActor :type Actor%20Object%20Reference) (ButtonPressed :type Key%20Structure :default "None"))
  (Development|PrintString (Utilities|GetDisplayName TouchedActor))
  (bind _asbp_test_player_controller (Utilities|Casting|CastToBP_TestPlayerController (Game|GetPlayerController 0)))
  (Default|TestRpc _asbp_test_player_controller TouchedActor))

(event EventBeginPlay
  (EventDispatchers|BindEventtoOnClicked (delegate Custom|OnClicked_Event)))

(event Collision|EventActorBeginOverlap
  (params (OtherActor :type Actor%20Object%20Reference)))

(event EventTick
  (params (DeltaSeconds :type Float%20%28single-precision%29)))

(fn ConstructionScript)

(fn OnRepRepBool
  (Development|PrintString (Utilities|String|Append (Utilities|String|ToString(Boolean) (Variables|Default|GetRepBool)) ", [nukxiong] OnRep")))

(fn OnRepRepActor
  (Development|PrintString (Utilities|String|Append (Utilities|GetDisplayName (Variables|Default|GetRepActor)) ", [nukxiong] OnRep")))