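; BP_TestPlayerController is a test player controller that binds number keys to spawn and exercise a BP_TestActor.
; Key 1 spawns the actor at an X offset from the controlled pawn and stores it as TestActor.
; Keys 2 and 3 call TestBlueprintCallable and TestComponent on that stored actor when it is valid.
; Disconnected nodes hold unused setup for a second linked actor with replication properties and a multicast call.
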(event Custom|Test
  (bind _returnvalue (Game|SpawnActorfromClass "/Game/Test/Blueprints/BP_TestActor.BP_TestActor_C" (Math|Conversions|ToTransform(Vector) (+ (Transformation|GetActorLocation (Pawn|GetControlledPawn)) "500.000000,0,0")) "Undefined" 0 0))
  (Variables|Default|SetTestActor _returnvalue))

(event Custom|MultiTest
  (bind _testactor (Variables|Default|GetTestActor))
  (Utilities|IsValid _testactor
    (:Is%20Valid
      (Class|TestActor|TestBlueprintCallable _testactor))))

(event Custom|TestComponent
  (bind _testactor (Variables|Default|GetTestActor))
  (Utilities|IsValid _testactor
    (:Is%20Valid
      (Class|TestActor|TestComponent _testactor))))

(event EventBeginPlay)

(event EventTick
  (params (DeltaSeconds :type Float%20%28single-precision%29)))

(event Input|KeyboardEvents|1
  (params (Key :type Key%20Structure :default "None"))
  (:Pressed
    (CallFunction|Test)))

(event Input|KeyboardEvents|2
  (params (Key :type Key%20Structure :default "None"))
  (:Pressed
    (CallFunction|MultiTest)))

(event Input|KeyboardEvents|3
  (params (Key :type Key%20Structure :default "None"))
  (:Pressed
    (CallFunction|TestComponent)))

(fn ConstructionScript)